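; BP_EnemySpawnPoint is an enemy spawner that runs timed waves from the location of its SpawnPoint component.
; After BeginPlay it waits StartDelay plus a fixed offset, then runs SpawnWaves.
; Three nested delayed loops walk WaveRules, each wave's EnemyOrder and each entry's spawn count, with timing read from the data.
; Each spawned enemy receives its entry's RestingRuleset and RouteIndex.
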(event Custom|Spawn%20Waves
  (bind _array_element (Utilities|ForEachLoopwithDelay (Variables|Default|Getwave%20rules) (.timeuntilnextwave (Utilities|Struct|BreakStruct_EnemyWave (stale _array_element))))
    (:LoopBody
      (bind _array_element_2 (Utilities|ForEachLoopwithDelay (.enemyorder (Utilities|Struct|BreakStruct_EnemyWave _array_element)) (.timebetweenspawns (Utilities|Struct|BreakStruct_EnemyWave_Order (stale _array_element_2))))
        (:LoopBody
          (Utilities|ForLoopwithDelay 1 (.number (Utilities|Struct|BreakStruct_EnemyWave_Order _array_element_2)) (.timeuntilnextspawn (Utilities|Struct|BreakStruct_EnemyWave_Order _array_element_2))
            (:LoopBody
              (Game|SpawnActorfromClass (.enemytype (Utilities|Struct|BreakStruct_EnemyWave_Order _array_element_2)) (Math|Transform|MakeTransform (Transformation|GetWorldLocation (Variables|Default|GetSpawn%20Point)) "0, 0, 0" "1.000000,1.000000,1.000000") "Undefined" "MultiplyWithRoot" 0 (.restingruleset (Utilities|Struct|BreakStruct_EnemyWave_Order _array_element_2)) (.routeindex (Utilities|Struct|BreakStruct_EnemyWave_Order _array_element_2)) 0))))))))

(event EventBeginPlay
  (Utilities|FlowControl|Delay (+ (Variables|Default|Getstart%20delay) 4.0))
  (CallFunction|SpawnWaves))

(fn ConstructionScript)