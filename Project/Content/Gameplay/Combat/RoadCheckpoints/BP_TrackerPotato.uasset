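; Enemy actor that walks a wave's road checkpoints toward its protection point, with optional timed rests along the way.
; After each stop it targets the nearest unpassed BP_RoadCheckpoint matching its WaveIndex, falling back to the matching BP_ProtectionPoint.
; Tick steps it by a fixed per-frame MovementSpeed unless resting, calculating or blocked.
; Overlapping a BP_Operator_2D passes the actor to that operator's BlockNewEnemy.
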(event OnComponentBeginOverlap(CollisionForBlocking)
  (params (OverlappedComponent :type Primitive%20Component%20Object%20Reference) (OtherActor :type Actor%20Object%20Reference) (OtherComp :type Primitive%20Component%20Object%20Reference) (OtherBodyIndex :type Integer) (bFromSweep :type Boolean) (SweepResult :type Hit%20Result%20Structure%20%28by%20ref%29))
  (bind _asbp_operator_2d (Utilities|Casting|CastToBP_Operator_2D OtherActor)
    (:then
      (Default|BlockNewEnemy _asbp_operator_2d self))
    (:CastFailed
      (Development|PrintString "Hello"))))

(event Custom|Move%20Towards%20Next%20Checkpoint
  (bind _defaultsceneroot (Variables|Default|GetDefaultSceneRoot))
  (bind _defaultsceneroot_2 (Variables|Default|GetDefaultSceneRoot))
  (bind _defaultsceneroot_3 (Variables|Default|GetDefaultSceneRoot))
  (bind _closest_checkpoint (Variables|Default|Getclosest%20checkpoint))
  (bind _returnvalue (Transformation|GetWorldLocation _defaultsceneroot))
  (bind _returnvalue_2 (Transformation|GetWorldRotation _defaultsceneroot_2))
  (bind _returnvalue_3 (Transformation|GetWorldLocation _defaultsceneroot_3))
  (bind _rootcomponent (Variables|/Script/Engine.Actor|GetRootComponent _closest_checkpoint))
  (bind _returnvalue_4 (Transformation|GetWorldLocation _rootcomponent))
  (if (<= (+ (Math|Float|Absolute(Float) (- (.x _returnvalue_4) (.x _returnvalue_3))) (Math|Float|Absolute(Float) (- (.y _returnvalue_4) (.y _returnvalue_3)))) 1e+01)
    (CallFunction|ReachedCheckpoint)
    (else
      (Transformation|SetWorldLocation (Variables|Default|GetDefaultSceneRoot) (+ _returnvalue (* (Math|Vector|GetForwardVector (Math|Rotator|MakeRotator (.roll _returnvalue_2) (.pitch _returnvalue_2) (+ (.yaw (Math|Rotator|FindLookatRotation _returnvalue (Transformation|GetWorldLocation (Variables|/Script/Engine.Actor|GetRootComponent (Variables|Default|Getclosest%20checkpoint))))) (.yaw _returnvalue_2)))) (Variables|Default|Getmovement%20speed))) false false))))

(event Custom|Reached%20Checkpoint
  (bind _resting_ruleset (Variables|Default|Getresting%20ruleset))
  (Variables|Default|Setresting true)
  (bind _result (Math|Integer|IncrementInt (Variables|Default|Getcurent%20reached%20checkpont))
    (:%20%20
      (if (Utilities|Array|IsValidIndex _resting_ruleset _result)
        (Utilities|FlowControl|Delay (Utilities|Array|Get(acopy) _resting_ruleset _result)))
      (Variables|Default|Setresting false)
      (CallFunction|GetClosestCheckpoint))))

(event EventTick
  (params (DeltaSeconds :type Float%20%28single-precision%29))
  (if (not (Math|Boolean|ORBoolean (Variables|Default|Getcalculating%20next%20distance?) (Variables|Default|Getresting) (Variables|Default|Getis%20blocked)))
    (CallFunction|MoveTowardsNextCheckpoint)))

(event EventBeginPlay
  (CallFunction|ReachedCheckpoint))

(fn ConstructionScript)

(fn GetClosestCheckpoint
  (Variables|Default|Setshortest%20route 9999.0)
  (Variables|Default|Setclosest%20checkpoint 0)
  (Variables|Default|Setalready%20passed%20? false)
  (Variables|Default|Setcalculating%20next%20distance? true)
  (bind _outactors (Actor|GetAllActorsOfClass "/Game/Gameplay/Combat/RoadCheckpoints/BP_RoadCheckpoint.BP_RoadCheckpoint_C"))
  (for _array_element _outactors
    (bind _array_element_2 (Utilities|Array|ForEachLoopwithBreak (Variables|Default|Getpassed%20actors) :!label _label)
      (:LoopBody
        (if (== _array_element_2 _array_element)
          (Variables|Default|Setalready%20passed%20? true)
          (goto _label Break)))
      (:Completed
        (if (not (Variables|Default|Getalready%20passed%20?))
          (bind _array_element_3 (Utilities|Array|ForEachLoopwithBreak (Utilities|Array|MakeArray (Variables|/Game/Gameplay/Combat/RoadCheckpoints/BP_RoadCheckpoint.BP_RoadCheckpoint_C|Getroute%20index _array_element)) :!label _label_2)
            (:LoopBody
              (if (== _array_element_3 (Variables|Default|Getwave%20index))
                (if (< (Transformation|GetDistanceTo _array_element) (Variables|Default|Getshortest%20route))
                  (Variables|Default|Setshortest%20route (Transformation|GetDistanceTo _array_element))
                  (Variables|Default|Setclosest%20checkpoint _array_element)
                  (goto _label_2 Break)))))))))
  (Variables|Default|Setcalculating%20next%20distance? false)
  (Utilities|Array|Add (Variables|Default|Getpassed%20actors) (Variables|Default|Getclosest%20checkpoint))
  (if (Utilities|IsValid (Variables|Default|Getclosest%20checkpoint))
    _
    (else
      (CallFunction|GetFinishPoint)))
  (return))

(fn GetFinishPoint
  (bind _outactors (Actor|GetAllActorsOfClass "/Game/Gameplay/Combat/ProtectionPoint/BP_ProtectionPoint.BP_ProtectionPoint_C"))
  (for _array_element _outactors
    (for _array_element_2 (Variables|/Game/Gameplay/Combat/ProtectionPoint/BP_ProtectionPoint.BP_ProtectionPoint_C|Getwave%20finish%20indexes _array_element)
      (if (== _array_element_2 (Variables|Default|Getwave%20index))
        (Variables|Default|Setclosest%20checkpoint _array_element)
        (return))))
  (Development|PrintString "Wrong index"))