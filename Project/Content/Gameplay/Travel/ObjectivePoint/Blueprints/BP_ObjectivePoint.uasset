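; Interactable stage marker for the travel map that shows stage details and opens the stage's level.
; On BeginPlay it reads completion and stars from GI_Global, turns completed beams green, unhides follow-up stages and builds the W_StageDetails widget.
; Interacting plays a sound and a timeline that scales up the 3D menu.
; Tick spins decorations and yaws the menu by the clamped Y offset to the travel camera.
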(event Custom|Rotate%20deco
  (Transformation|AddRelativeRotation (Variables|Default|GetDeco1) "0.000000,0.100000,0.000000" false false)
  (Transformation|AddRelativeRotation (Variables|Default|GetDeco) "0.000000,0.200000,0.000000" false false)
  (Transformation|AddRelativeRotation (Variables|Default|GetDeco%202) "0.000000,0.300000,0.000000" false false))

(event Custom|Rotate%20towards%20player
  (bind _asbp_camera_controller_travel (Utilities|Casting|CastToBP_CameraController_Travel (Game|Player|GetPlayerPawn 0)))
  (Transformation|SetRelativeRotation (Variables|Default|GetSM_Menu) (Math|Rotator|MakeRotator 0.0 0.0 (Math|Float|Clamp(Float) (- (.y (Transformation|GetWorldLocation (Variables|/Game/Player/Blueprints/Travel/BP_CameraController_Travel.BP_CameraController_Travel_C|GetCamera _asbp_camera_controller_travel))) (.y (Transformation|GetWorldLocation (Variables|Default|GetDefaultSceneRoot)))) -6e+01 2e+01)) false false))

(event Custom|Set%20info%20widget
  (bind _returnvalue (UserInterface|CreateWidget "/Game/Gameplay/Travel/ObjectivePoint/Widgets/W_StageDetails.W_StageDetails_C" 0 (Variables|Default|GetStage%20Id) (Variables|Default|GetStage%20Name) (Variables|Default|GetStars%20Gotten) (Variables|Default|GetStage%20Image) (Variables|Default|GetFirst%20Clear%20Rewards%20Text) (Variables|Default|GetAdditional%20Rewards%20Text)))
  (Variables|Default|SetInfo%20Widget _returnvalue))

(event Custom|Open%20Info%20Widget
  (bind _info_widget (Variables|Default|GetInfo%20Widget))
  (UserInterface|Viewport|AddtoViewport _info_widget 0)
  (Default|OpenWidget _info_widget))

(event Custom|Close%20Info%20Widget
  (bind _info_widget (Variables|Default|GetInfo%20Widget))
  (Default|CloseWidget _info_widget)
  (Widget|RemovefromParent _info_widget))

(event Custom|Start%20Stage
  (Game|OpenLevel(byObjectReference) (Variables|Default|GetLevel)))

(event Custom|Set%20data%20from%20game%20instance
  (bind _asgi_global (Utilities|Casting|CastToGI_Global (Game|GetGameInstance)))
  (bind (_completed__ _stars) (Default|GetStageData _asgi_global (Variables|Default|GetId)))
  (bind _output_get (Variables|Default|Setcompleted%20stage%20? _completed__))
  (Variables|Default|SetStars%20Gotten _stars)
  (Utilities|FlowControl|Sequence
    (:then_0
      (if _output_get
        (Rendering|Material|SetMaterial (Variables|Default|GetSM_LightBeam) 0 "/Game/Gameplay/Travel/ObjectivePoint/Materials/MI_Glow_Green.MI_Glow_Green")
        (CallFunction|UnlockNextStages)))
    (:then_1
      (CallFunction|SetInfoWidget))))

(event Custom|Unlock%20Next%20Stages
  (bind _unlocked_stages_after_completion (Variables|Default|Getunlocked%20stages%20after%20completion))
  (if (> (Utilities|Array|Length _unlocked_stages_after_completion) 0)
    (for _array_element _unlocked_stages_after_completion
      (Rendering|SetActorHiddenInGame _array_element false))))

(event EventBeginPlay
  (Components|Timeline|SetPlayRate (Variables|Default|GetOpen%20/%20Close%20Menu) (/ 1.0 (Variables|Default|Gettime%20to%20open%20menu)))
  (Transformation|SetWorldScale3D (Variables|Default|GetSM_Menu) "0.010000,0.010000,0.010000")
  (CallFunction|SetDatafromGameInstance)
  (if (Variables|Default|Getis%20unlocked%20from%20start%20?)
    (Rendering|SetActorHiddenInGame false)))

(event EventTick
  (params (DeltaSeconds :type Float%20%28single-precision%29))
  (CallFunction|RotateDeco)
  (CallFunction|RotateTowardsPlayer))

(event Custom|Handle%20Interaction
  (if (not (Variables|Default|Getis%20menu%20open%20?))
    (CallFunction|OpenMenu)))

(event Custom|Close%20Menu
  (Variables|Default|Setis%20menu%20open%20? false)
  (bind _newtrack_0 (Timeline|Open%20/%20Close%20Menu Reverse)
    (:Update
      (Transformation|SetWorldScale3D (Variables|Default|GetSM_Menu) (Math|Conversions|ToVector(Float) _newtrack_0)))))

(event Custom|Open%20Menu
  (Variables|Default|Setis%20menu%20open%20? true)
  (Audio|PlaySound2D "/Game/Gameplay/Travel/ObjectivePoint/SFX/mixkit-retro-arcade-casino-notification-211.mixkit-retro-arcade-casino-notification-211" 1.0 1.0 0.3 0 0)
  (bind _newtrack_0 (Timeline|Open%20/%20Close%20Menu Play)
    (:Update
      (Transformation|SetWorldScale3D (Variables|Default|GetSM_Menu) (Math|Conversions|ToVector(Float) _newtrack_0)))))

(fn ConstructionScript)

(fn EndInteraction
  (params (instigator :type Actor%20Object%20Reference))
  (return false))

(fn Interact
  (params (instigator :type Actor%20Object%20Reference))
  (CallFunction|HandleInteraction)
  (return false))