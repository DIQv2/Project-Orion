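; Camera controller for the Travel mode: a mouse-driven view that pans and picks objects under the cursor.
; On begin play it shows the cursor, enables touch events and creates the main travel UI widget.
; Holding left mouse drags a swept Sphere by the frame-to-frame cursor delta.
; A shared deprojected cursor trace drives click interaction through I_Interactable and per-tick hover toggling on objective point buttons.
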(event EventBeginPlay
  (bind _returnvalue (Game|GetPlayerController 0))
  (bind _output_get (Variables|/Script/Engine.PlayerController|SetbShowMouseCursor _returnvalue true))
  (Variables|/Script/Engine.PlayerController|SetbEnableTouchEvents _returnvalue _output_get)
  (CallFunction|InitMainWidget))

(event EventTick
  (params (DeltaSeconds :type Float%20%28single-precision%29))
  (CallFunction|Movement)
  (CallFunction|TraceCursor))

(event Input|ActionEvents|InputActionLeftClick
  (params (Key :type Key%20Structure))
  (:Pressed
    (bind _returnvalue (Class|WidgetLayoutLibrary|GetMousePositiononViewport))
    (Variables|Default|SetprevieousTouchLocation _returnvalue)
    (bind (_hit_location _hit _hit_actor) (CallFunction|LineTracefromCursor 0 "TraceTypeQuery1"))
    (if _hit
      (bind _asi_interactable (Utilities|Casting|CastToI_Interactable _hit_actor))
      (Default|Interact _asi_interactable))))

(event Custom|Movement
  (if (Game|Player|IsInputKeyDown (Game|GetPlayerController 0) "LeftMouseButton")
    (bind _returnvalue (Class|WidgetLayoutLibrary|GetMousePositiononViewport))
    (Variables|Default|SetnewTouchLocation _returnvalue)
    (Transformation|AddWorldOffset (Variables|Default|GetSphere) (Math|Vector|MakeVector (.y (- (Variables|Default|GetnewTouchLocation) (Variables|Default|GetprevieousTouchLocation))) (* (.x (- (Variables|Default|GetnewTouchLocation) (Variables|Default|GetprevieousTouchLocation))) -1.0) 0.0) true false)
    (Variables|Default|SetprevieousTouchLocation (Variables|Default|GetnewTouchLocation))))

(event Custom|Trace%20Cursor
  (bind _hit_actor (CallFunction|LineTracefromCursor 0 "TraceTypeQuery1"))
  (bind _asbp_objective_point_button (Utilities|Casting|CastToBP_ObjectivePoint_Button _hit_actor)
    (:then
      (if (not (== _asbp_objective_point_button (Variables|Default|Getcurrent%20hovered%20button)))
        (Utilities|IsValid (Variables|Default|Getcurrent%20hovered%20button)
          (:Is%20Valid
            (Default|EndHover (Variables|Default|Getcurrent%20hovered%20button)))
          (:Is%20Not%20Valid
            _))
        (bind _output_get (Variables|Default|Setcurrent%20hovered%20button _asbp_objective_point_button))
        (Default|Hover _output_get)))
    (:CastFailed
      (Utilities|IsValid (Variables|Default|Getcurrent%20hovered%20button)
        (:Is%20Valid
          (Default|EndHover (Variables|Default|Getcurrent%20hovered%20button))
          (Variables|Default|Setcurrent%20hovered%20button 0))))))

(event Custom|Init%20Main%20Widget
  (bind _returnvalue (UserInterface|CreateWidget "/Game/Player/Blueprints/Travel/Widgets/W_MainTravelUI.W_MainTravelUI_C"))
  (UserInterface|Viewport|AddtoViewport _returnvalue 0))

(fn ConstructionScript)

(fn LineTracefromCursor
  (params (actors%20to%20ignore :type Array%20of%20Actor%20Object%20References) (Trace%20channel :type ETraceTypeQuery%20Enum :default "TraceTypeQuery1"))
  (bind _returnvalue (Game|GetPlayerController 0))
  (bind (_worldlocation _worlddirection) (Game|Player|ConvertMouseLocationToWorldSpace _returnvalue))
  (bind (_outhit _returnvalue_2) (Collision|LineTraceByChannel _worldlocation (+ _worldlocation (* _worlddirection 1e+04)) Trace%20channel false actors%20to%20ignore "None"))
  (return (.Location (Collision|BreakHitResult _outhit)) _returnvalue_2 (.HitActor (Collision|BreakHitResult _outhit)) (.HitComponent (Collision|BreakHitResult _outhit)) (.HitItem (Collision|BreakHitResult _outhit))))