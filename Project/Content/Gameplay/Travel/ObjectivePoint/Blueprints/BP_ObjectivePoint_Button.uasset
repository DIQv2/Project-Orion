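; Objective point button in the travel gameplay that gives animated and audio feedback when hovered.
; Hover plays a sound and runs a Timeline that raises the static mesh and scales it up from the relative transform cached at BeginPlay.
; EndHover reverses the same Timeline to ease the mesh back.
; Its Interact function only returns false, with no logic of its own.
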(event Custom|End%20Hover
  (bind _initial_relative_transform (Variables|Default|GetInitial%20Relative%20Transform))
  (bind _newtrack_0 (Timeline|Timeline Reverse)
    (:Update
      (Transformation|SetRelativeTransform (Variables|Default|GetStaticMesh) (Math|Transform|MakeTransform (Math|Vector|MakeVector (.x (.location _initial_relative_transform)) (.y (.location _initial_relative_transform)) (+ (* _newtrack_0 1e+01) (.z (.location _initial_relative_transform)))) (.rotation _initial_relative_transform) (+ (* _newtrack_0 0.4) (.scale _initial_relative_transform))) false false))))

(event Custom|Hover
  (bind _initial_relative_transform (Variables|Default|GetInitial%20Relative%20Transform))
  (Audio|PlaySound2D "/Game/Gameplay/Travel/ObjectivePoint/SFX/SC_ButtonHover.SC_ButtonHover" 1.0 1.0 0.2 0 0)
  (bind _newtrack_0 (Timeline|Timeline Play)
    (:Update
      (Transformation|SetRelativeTransform (Variables|Default|GetStaticMesh) (Math|Transform|MakeTransform (Math|Vector|MakeVector (.x (.location _initial_relative_transform)) (.y (.location _initial_relative_transform)) (+ (* _newtrack_0 1e+01) (.z (.location _initial_relative_transform)))) (.rotation _initial_relative_transform) (+ (* _newtrack_0 0.4) (.scale _initial_relative_transform))) false false))))

(event EventBeginPlay
  (Variables|Default|SetInitial%20Relative%20Transform (Transformation|GetRelativeTransform (Variables|Default|GetStaticMesh))))

(fn ConstructionScript
  (|CallParentFunction))

(fn Interact
  (params (instigator :type Actor%20Object%20Reference))
  (return false))