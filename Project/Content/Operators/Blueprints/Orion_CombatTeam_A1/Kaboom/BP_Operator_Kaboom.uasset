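; Operator Blueprint for Kaboom that implements the operator's skill effects.
; Skill activation and deactivation events switch on the selected skill in the Stats struct, with only the first skill handled.
; That skill halves the attack interval while active, and deactivation writes back a hard-coded value rather than a saved one.
; BeginPlay, overlap, Tick and the construction script add no logic of their own.
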(event Custom|Activate%201st%20Skill
  (Utilities|Struct|SetmembersinStruct_OperatorData (Variables|Default|Getstats) 1.0))

(event Custom|Deactivate%201st%20Skill%20Effects
  (Utilities|Struct|SetmembersinStruct_OperatorData (Variables|Default|Getstats) 2.0))

(event EventBeginPlay
  (|CallParentFunction) ; This node is disabled and will not be called.\nDrag off pins to build functionality.
)

(event Collision|EventActorBeginOverlap
  (params (OtherActor :type Actor%20Object%20Reference)))

(event EventTick
  (params (DeltaSeconds :type Float%20%28single-precision%29))
  (|CallParentFunction DeltaSeconds) ; This node is disabled and will not be called.\nDrag off pins to build functionality.
)

(event EventActivateSkillEffects
  (switch int (Utilities|Struct|BreakStruct_OperatorData (Variables|Default|Getstats))
    (:0
      (CallFunction|Activate1stSkill))))

(event EventDeactivateSkillEffects
  (switch int (Utilities|Struct|BreakStruct_OperatorData (Variables|Default|Getstats))
    (:0
      (CallFunction|Deactivate1stSkillEffects))))

(fn ConstructionScript
  (|CallParentFunction))