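; Scout operator Blueprint for a deployment-based combat game, overriding skill behavior from its parent operator class.
; Activating the first skill jumps the animation to "Special" and clears range actors, enemies in range, blocked enemies and the attack target.
; Ending the skill deactivates it and grants deployment points through the StageHandler, capped at the maximum.
; Deactivating the first skill's effects rebuilds the attack range and hides its display.
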(event Custom|Deactivate%20Skill%201%20Effects
  (CallFunction|CalculateRange)
  (CallFunction|HideRange))

(event Custom|End%20Skill
  (bind _stage_handler (Variables|Default|Getstage%20handler))
  (CallFunction|DeactivateSkill)
  (Variables|/Game/Gameplay/Combat/GameHandler/Blueprints/BP_StageHandler.BP_StageHandler_C|Setdeployment%20points _stage_handler (Math|Float|Min(Float) (+ (Variables|/Game/Gameplay/Combat/GameHandler/Blueprints/BP_StageHandler.BP_StageHandler_C|Getdeployment%20points _stage_handler) 12.0) (Math|Conversions|ToFloat(Integer) (Variables|/Game/Gameplay/Combat/GameHandler/Blueprints/BP_StageHandler.BP_StageHandler_C|Getmax%20dp _stage_handler)))))

(event Custom|Activate%201st%20Skill%20Effects
  (Class|PaperZDAnimInstance|JumptoNode (Variables|/Script/PaperZD.PaperZDAnimationComponent|GetAnimInstance (Variables|Default|GetAnimationComponent)) "Special" "None")
  (CallFunction|DestroyandEmptyRangeActors)
  (Utilities|Array|Clear (Variables|Default|Getenemies%20in%20range))
  (Utilities|Array|Clear (Variables|Default|Getblocked%20enemies))
  (Variables|Default|Setactor%20to%20attack 0))

(event EventBeginPlay
  (|CallParentFunction) ; This node is disabled and will not be called.\nDrag off pins to build functionality.
)

(event Collision|EventActorBeginOverlap
  (params (OtherActor :type Actor%20Object%20Reference)))

(event EventTick
  (params (DeltaSeconds :type Float%20%28single-precision%29))
  (|CallParentFunction DeltaSeconds) ; This node is disabled and will not be called.\nDrag off pins to build functionality.
)

(event EventActivateSkillEffects
  (switch int (Utilities|Struct|BreakStruct_OperatorData (Variables|Default|Getstats))
    (:0
      (CallFunction|Activate1stSkillEffects))))

(event EventDeactivateSkillEffects
  (switch int (Utilities|Struct|BreakStruct_OperatorData (Variables|Default|Getstats))
    (:0
      (CallFunction|DeactivateSkill1Effects))))

(fn ConstructionScript
  (|CallParentFunction))