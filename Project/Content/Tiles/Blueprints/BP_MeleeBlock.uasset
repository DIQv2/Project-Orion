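; BP_MeleeBlock is a tile block that tracks whether it is free and can show or hide a highlight.
; ChangeState writes the IsFree flag and GetState returns it.
; Highlight and Unhighlight toggle the HighlightMesh component's hidden-in-game state, without propagating to children.
; The construction script is empty, and the file contains no logic that decides when the state or highlight changes.
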(fn ConstructionScript)

(fn ChangeState
  (params (is%20free%20? :type Boolean))
  (Variables|Default|Setis%20free? is%20free%20?)
  (return false))

(fn GetState
  (return (Variables|Default|Getis%20free?)))

(fn Highlight
  (Development|SetHiddeninGame (Variables|Default|GetHighlightMesh) false false)
  (return false))

(fn Unhighlight
  (Development|SetHiddeninGame (Variables|Default|GetHighlightMesh) true false)
  (return false))