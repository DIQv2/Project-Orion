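; Stage handler for a wave-based defense mission, tracking lives, enemy kills, deployment points and the win or loss result.
; On BeginPlay it initializes the level, totals enemies from spawn-point wave rules, then shows the HUD and starts timer-driven deployment point regeneration.
; Kill and breach events update the HUD and trigger stage completion or failure.
; Completion rates stars by remaining lives, grants XP and saves the result to GI_Global.
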(event Custom|Stage%20Fail
  (Variables|Runtime|Setlost%20? false)
  (Game|SetGamePaused true)
  (bind _returnvalue (UserInterface|CreateWidget "/Game/Gameplay/Combat/GameHandler/Widgets/W_StageLoss.W_StageLoss_C" 0 self))
  (UserInterface|Viewport|AddtoViewport _returnvalue 0))

(event Custom|End%20stage%20and%20Return%20to%20world
  (Default|EndStage (Variables|Default|Getgame%20instance))
  (Game|OpenLevel(byObjectReference) (Variables|Init|GetLevel)))

(event Custom|Stage%20Complete
  (bind _game_instance (Variables|Default|Getgame%20instance))
  (bind _total_lives (Variables|Constants|Gettotal%20lives))
  (bind _lives (Variables|Runtime|Getlives))
  (bind _returnvalue (/ _lives _total_lives))
  (bind _returnvalue_2 (* _returnvalue 1e+02))
  (Utilities|FlowControl|Sequence
    (:then_0
      (if (> _returnvalue_2 5e+01)
        (Math|Integer|IncrementInt (Variables|Runtime|Getstars)
          (:%20%20
            (if (== _returnvalue_2 1e+02)
              (Math|Integer|IncrementInt (Variables|Runtime|Getstars)))))))
    (:then_1
      (Utilities|FlowControl|Delay 1.0)
      (if (not (Variables|Runtime|Getlost%20?))
        (Game|SetGamePaused true)
        (bind _returnvalue_3 (UserInterface|CreateWidget "/Game/Gameplay/Combat/GameHandler/Widgets/W_StageWin.W_StageWin_C" 0 (Variables|Init|GetMission%20Name) (Variables|Init|GetMission%20Id) (* (/ (Variables|Runtime|Getlives) (Variables|Constants|Gettotal%20lives)) 1e+02) self))
        (UserInterface|Viewport|AddtoViewport _returnvalue_3 0)
        (bind _stars (Default|GetStageData _game_instance (Variables|Init|GetId)))
        (if (and (== _stars 0) (== (Variables|Runtime|Getstars) 3))
          (CallFunction|GiveFirstClearXP)
          (else
            (CallFunction|GiveStageXP)))
        (Default|AddStageData _game_instance (Variables|Init|GetId) (Variables|Runtime|Getstars))))))

(event Custom|Give%20Stage%20XP
  (Default|AddPlayerXP (Variables|Default|Getgame%20instance) (Math|Float|Truncate (* (Variables|Default|Getreward%20xp) 0.3)))
  (CallFunction|GiveAdditionalRewards))

(event Custom|Give%20First%20Clear%20XP
  (Default|AddPlayerXP (Variables|Default|Getgame%20instance) (Variables|Default|Getreward%20xp))
  (CallFunction|GiveAdditionalRewards))

(event Custom|Give%20Additional%20Rewards
  ;[1 1 1] For custom
)

(event EventBeginPlay
  (Utilities|FlowControl|Sequence
    (:then_0
      (Utilities|InitializeCombatLevel (Variables|Init|GetBGM) (Variables|Init|GetMission%20Name) (Variables|Init|GetMission%20Id)
        (:Continue
          (Variables|Runtime|Setlives (Variables|Constants|Gettotal%20lives))
          (bind _asgi_global (Utilities|Casting|CastToGI_Global (Game|GetGameInstance)))
          (bind _output_get (Variables|Default|Setgame%20instance _asgi_global))
          (Default|StartStage _output_get)
          (Variables|runtime|Setdeployment%20points (Math|Conversions|ToFloat(Integer) (Variables|Constants|Getinitial%20deployment%20points))))))
    (:then_1
      (bind _outactors (Actor|GetAllActorsOfClass "/Game/Gameplay/Combat/EnemySpawn/Blueprint/BP_EnemySpawnPoint.BP_EnemySpawnPoint_C"))
      (for _array_element _outactors
        (for _array_element_2 (Variables|/Game/Gameplay/Combat/EnemySpawn/Blueprint/BP_EnemySpawnPoint.BP_EnemySpawnPoint_C|Getwave%20rules _array_element)
          (for _array_element_3 (Utilities|Struct|BreakStruct_EnemyWave _array_element_2)
            (Variables|Runtime|Settotal%20enemies (+ (Utilities|Struct|BreakStruct_EnemyWave_Order _array_element_3) (Variables|Runtime|Gettotal%20enemies)))))))
    (:then_2
      (Utilities|FlowControl|Delay 4.0)
      (bind _returnvalue (UserInterface|CreateWidget "/Game/Gameplay/Combat/GameHandler/Widgets/W_StageData.W_StageData_C" 0 (Utilities|Text|ToText(Integer) (Variables|Runtime|Getlives)) (Utilities|Text|ToText(Integer) (Variables|Runtime|Gettotal%20enemies)) (Utilities|Text|ToText(Integer) (Variables|Runtime|Getenemies%20killed))))
      (bind _output_get_2 (Variables|Init|Setwidget _returnvalue))
      (UserInterface|Viewport|AddtoViewport _output_get_2 0)
      (CallFunction|InitDPRegen))))

(event EventEnemyEliminated
  (bind _result (Math|Integer|IncrementInt (Variables|Runtime|Getenemies%20killed))
    (:%20%20
      (Variables|/Game/Gameplay/Combat/GameHandler/Widgets/W_StageData.W_StageData_C|Setenemies%20killed (Variables|Init|Getwidget) (Utilities|Text|ToText(Integer) _result))
      (if (>= _result (Variables|Runtime|Gettotal%20enemies))
        (CallFunction|StageComplete)))))

(event EventEnemyEnteredProtectionPoint
  (bind _widget (Variables|Init|Getwidget))
  (bind _result (Math|Integer|DecrementInt (Variables|Runtime|Getlives))
    (:%20%20
      (Variables|/Game/Gameplay/Combat/GameHandler/Widgets/W_StageData.W_StageData_C|Setlives _widget (Utilities|Text|ToText(Integer) (Math|Integer|Max(Integer) _result)))
      (Default|LifePointsBlink _widget)
      (if (<= _result 0)
        (CallFunction|StageFail)))))

(fn ConstructionScript)

(fn RegenerateDP
  (Variables|runtime|Setdeployment%20points (Math|Float|Clamp(Float) (+ (Variables|runtime|Getdeployment%20points) (Variables|Runtime|Getdp%20regen%20amount)) 0.0 (Math|Conversions|ToFloat(Integer) (Variables|constants|Getmax%20dp)))))

(fn InitDPRegen
  (switch Utilities|FlowControl|Switch|SwitchonEnum_DpRegenType (Variables|Init|Getdp%20regen%20type)
    (:NewEnumerator0
      (Variables|Runtime|Setdp%20regen%20amount 0.08))
    (:NewEnumerator1
      (Variables|Runtime|Setdp%20regen%20amount 0.05))
    (:NewEnumerator2
      (Variables|Runtime|Setdp%20regen%20amount 0.03)))
  (Utilities|Time|SetTimerbyFunctionName 0 "Regenerate DP" 0.05 true))