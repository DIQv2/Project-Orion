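; Grenade projectile that explodes on hit, damaging enemies caught in its blast and spawning an explosion actor and sound.
; On hit, it sets two blast volumes (AOEExplosion, InnerExplosion) to overlap a custom collision channel, stops moving, then destroys itself.
; Each volume's begin-overlap event damages BP_Enemy actors with the same multiplier, so enemies overlapping both can be damaged twice.
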(event OnComponentBeginOverlap(AOEExplosion)
  (params (OverlappedComponent :type Primitive%20Component%20Object%20Reference) (OtherActor :type Actor%20Object%20Reference) (OtherComp :type Primitive%20Component%20Object%20Reference) (OtherBodyIndex :type Integer) (bFromSweep :type Boolean) (SweepResult :type Hit%20Result%20Structure%20%28by%20ref%29))
  (bind _asbp_enemy (Utilities|Casting|CastToBP_Enemy OtherActor))
  (CallFunction|DealDamagetoEnemy 2.5 _asbp_enemy))

(event OnComponentBeginOverlap(InnerExplosion)
  (params (OverlappedComponent :type Primitive%20Component%20Object%20Reference) (OtherActor :type Actor%20Object%20Reference) (OtherComp :type Primitive%20Component%20Object%20Reference) (OtherBodyIndex :type Integer) (bFromSweep :type Boolean) (SweepResult :type Hit%20Result%20Structure%20%28by%20ref%29))
  (bind _asbp_enemy (Utilities|Casting|CastToBP_Enemy OtherActor))
  (CallFunction|DealDamagetoEnemy 2.5 _asbp_enemy))

(event EventBeginPlay
  (|CallParentFunction) ; This node is disabled and will not be called.\nDrag off pins to build functionality.
)

(event Collision|EventActorBeginOverlap
  (params (OtherActor :type Actor%20Object%20Reference)))

(event EventTick
  (params (DeltaSeconds :type Float%20%28single-precision%29)))

(event EventEventonHit
  (Collision|SetCollisionResponsetoChannel (Variables|Default|GetAOE%20Explosion) "ECC_GameTraceChannel6" "ECR_Overlap")
  (Variables|/Script/Engine.MovementComponent|SetVelocity (Variables|Default|GetProjectileMovement) "0, 0, 0")
  (Game|SpawnActorfromClass "/Game/VFX/FXVarietyPack/Blueprints/BP_ky_explosion.BP_ky_explosion_C" (Transformation|GetActorTransform) "Undefined" "MultiplyWithRoot" 0 0)
  (Audio|PlaySound2D "/Game/SFX/Grenade/SC_GrenadeExplosion.SC_GrenadeExplosion" 1.0 1.0 0.0 0 0)
  (Actor|DestroyActor))

(fn ConstructionScript
  (|CallParentFunction))