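; Base projectile that launches on BeginPlay at the spawn-time location of an enemy or operator target.
; A suggested toss velocity, fixed-speed or custom-arc, drives ProjectileMovement, and only overlap with that target counts as a hit.
; Hits fire OnHit for children, then non-AoE shots subtract Damage from Health, capped at max HP.
; AoE shots skip damage, and on enemy hits also skip self-destruction.
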(event OnComponentBeginOverlap(hitcollision)
  (params (OverlappedComponent :type Primitive%20Component%20Object%20Reference) (OtherActor :type Actor%20Object%20Reference) (OtherComp :type Primitive%20Component%20Object%20Reference) (OtherBodyIndex :type Integer) (bFromSweep :type Boolean) (SweepResult :type Hit%20Result%20Structure%20%28by%20ref%29))
  (if (== OtherActor (Variables|Default|GetEnemyTarget))
    (CallFunction|HandleHittingEnemyTarget)
    (elif (== OtherActor (Variables|Default|GetOperatorTarget))
      (CallFunction|HandleHittingOperatorTarget))))

(event Custom|Shoot%20towards%20target
  (params (target :type Actor%20Object%20Reference))
  (if (not (Variables|Default|Getarched%20?))
    (bind _tossvelocity (Class|GameplayStatics|BlueprintSuggestProjectileVelocity (Transformation|GetWorldLocation (Variables|Default|GetDefaultSceneRoot)) (Variables|Default|Gettarget%20location) (Variables|Default|Getspeed) 0.0 "DoNotTrace" 0.0 false false true))
    (Variables|/Script/Engine.MovementComponent|SetVelocity (Variables|Default|GetProjectileMovement) _tossvelocity)
    (else
      (bind _outlaunchvelocity (Game|SuggestProjectileVelocityCustomArc (Transformation|GetWorldLocation (Variables|Default|GetDefaultSceneRoot)) (Variables|Default|Gettarget%20location) 0.0 (Variables|Default|Getarc%20param)))
      (Variables|/Script/Engine.MovementComponent|SetVelocity (Variables|Default|GetProjectileMovement) _outlaunchvelocity))))

(event Custom|Handle%20Hitting%20Enemy%20Target
  (CallFunction|EventonHit)
  (if (not (Variables|Default|Getaoe%20?))
    (CallFunction|DealDamagetoEnemy 1.0 (Variables|Default|GetEnemyTarget))
    (Actor|DestroyActor)))

(event Custom|Handle%20Hitting%20Operator%20Target
  (bind _operatortarget (Variables|Default|GetOperatorTarget))
  (CallFunction|EventonHit)
  (if (not (Variables|Default|Getaoe%20?))
    (Utilities|IsValid _operatortarget
      (:Is%20Valid
        (Variables|/Game/Operators/Blueprints/BP_Operator_2D.BP_Operator_2D_C|Sethealth _operatortarget (Math|Float|Min(Float) (- (Variables|/Game/Operators/Blueprints/BP_Operator_2D.BP_Operator_2D_C|Gethealth _operatortarget) (Variables|Default|Getdamage)) (Utilities|Struct|BreakStruct_OperatorData (Variables|/Game/Operators/Blueprints/BP_Operator_2D.BP_Operator_2D_C|Getstats _operatortarget)))))))
  (Actor|DestroyActor))

(event Custom|Event%20on%20hit
  ;[0.04062 0.04062 0.04062] For children
)

(event Custom|Deal%20damage%20to%20enemy
  (params (damage%20multiplier :type Float%20%28double-precision%29) (Enemy :type BP%20Enemy%20Object%20Reference))
  (Utilities|IsValid Enemy
    (:Is%20Valid
      (if (> (Variables|/Game/Enemies/Blueprints/BP_Enemy.BP_Enemy_C|Gethealth Enemy) 0.0)
        (Variables|/Game/Enemies/Blueprints/BP_Enemy.BP_Enemy_C|Sethealth Enemy (Math|Float|Min(Float) (- (Variables|/Game/Enemies/Blueprints/BP_Enemy.BP_Enemy_C|Gethealth Enemy) (* damage%20multiplier (Variables|Default|Getdamage))) (.HP (Utilities|Struct|BreakStruct_EnemyStats (Variables|/Game/Enemies/Blueprints/BP_Enemy.BP_Enemy_C|Getstats Enemy)))))))))

(event EventBeginPlay
  (bind _operatortarget (Variables|Default|GetOperatorTarget))
  (bind _enemytarget (Variables|Default|GetEnemyTarget))
  (Utilities|IsValid _enemytarget
    (:Is%20Valid
      (Variables|Default|Settarget%20location (Transformation|GetWorldLocation (Variables|/Script/Paper2D.PaperCharacter|GetSprite _enemytarget)))
      (CallFunction|ShootTowardsTarget _enemytarget))
    (:Is%20Not%20Valid
      (Utilities|IsValid _operatortarget
        (:Is%20Valid
          (Variables|Default|Settarget%20location (Transformation|GetWorldLocation (Variables|/Script/Paper2D.PaperCharacter|GetSprite _operatortarget)))
          (CallFunction|ShootTowardsTarget _operatortarget))))))

(fn ConstructionScript)