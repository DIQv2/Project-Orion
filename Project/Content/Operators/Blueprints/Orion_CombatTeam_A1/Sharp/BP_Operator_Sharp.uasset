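; Operator Blueprint for Sharp, implementing three selectable skills dispatched on Stats.SelectedSkill when skill effects activate or deactivate.
; Skill one temporarily boosts ATK and speeds the actor up through CustomTimeDilation.
; Skill two polls until an enemy is in range, plays a grenade animation, and ThrowGrenade fires a projectile and ends the skill.
; Skill three switches subclass and explosive projectile and extends range; deactivation resets subclass and range, but not projectile class.
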(event Custom|Throw%20Grenade
  (CallFunction|ProjectileAttackPattern 1.0)
  (CallFunction|DeactivateSkill))

(event Custom|Activate%202nd%20Skill
  (if (not (Variables|Default|Gethas%20thrown%20grenade))
    (if (> (Utilities|Array|Length (Variables|Default|Getenemies%20in%20range)) 0)
      (Variables|Default|Sethas%20thrown%20grenade true)
      (Class|PaperZDAnimInstance|JumptoNode (Variables|/Script/PaperZD.PaperZDAnimationComponent|GetAnimInstance (Variables|Default|GetAnimationComponent)) "Throw Grenade" "None")
      (else
        (Utilities|FlowControl|Delay 0.1)
        (CallFunction|ActivateSkillEffects)))))

(event Custom|Activate%201st%20Skill
  (bind _stats (Variables|Default|Getstats))
  (Utilities|Struct|SetmembersinStruct_OperatorData _stats (* (Utilities|Struct|BreakStruct_OperatorData _stats) 1.2))
  (Variables|Default|SetCustomTimeDilation 1.2))

(event Custom|Deactivate%201st%20Skill%20Effects
  (bind _stats (Variables|Default|Getstats))
  (Utilities|Struct|SetmembersinStruct_OperatorData _stats (/ (Utilities|Struct|BreakStruct_OperatorData _stats) 1.2))
  (Variables|Default|SetCustomTimeDilation 1.0))

(event Custom|Deactivate%202nd%20Skill%20Effects
  (Variables|Default|Sethas%20thrown%20grenade false))

(event Custom|Activate%203rd%20Skill
  (Utilities|Struct|SetmembersinStruct_OperatorType (Variables|Default|Getclass) "NewEnumerator10" "/Game/Projectiles/Blueprints/ExplosiveBullet/BP_ExplosiveBullet.BP_ExplosiveBullet_C")
  (Utilities|Array|Add (Variables|Default|Getrange) "(X=4.000000,Y=1.000000)")
  (CallFunction|DestroyandEmptyRangeActors)
  (CallFunction|CalculateRange)
  (CallFunction|HideRange))

(event Custom|Deactivate%203rd%20Skill%20Effects
  (Utilities|Struct|SetmembersinStruct_OperatorType (Variables|Default|Getclass) "NewEnumerator2")
  (Utilities|Array|RemoveIndex (Variables|Default|Getrange) 4)
  (CallFunction|DestroyandEmptyRangeActors)
  (CallFunction|CalculateRange)
  (CallFunction|HideRange))

(event EventBeginPlay
  (|CallParentFunction) ; This node is disabled and will not be called.\nDrag off pins to build functionality.
)

(event Collision|EventActorBeginOverlap
  (params (OtherActor :type Actor%20Object%20Reference)))

(event EventTick
  (params (DeltaSeconds :type Float%20%28single-precision%29))
  (|CallParentFunction DeltaSeconds) ; This node is disabled and will not be called.\nDrag off pins to build functionality.
)

(event EventActivateSkillEffects
  (switch int (Utilities|Struct|BreakStruct_OperatorData (Variables|Default|Getstats))
    (:0
      (CallFunction|Activate1stSkill))
    (:1
      (CallFunction|Activate2ndSkill))
    (:2
      (CallFunction|Activate3rdSkill))))

(event EventDeactivateSkillEffects
  (switch int (Utilities|Struct|BreakStruct_OperatorData (Variables|Default|Getstats))
    (:0
      (CallFunction|Deactivate1stSkillEffects))
    (:1
      (CallFunction|Deactivate2ndSkillEffects))
    (:2
      (CallFunction|Deactivate3rdSkillEffects))))

(fn ConstructionScript
  (|CallParentFunction))