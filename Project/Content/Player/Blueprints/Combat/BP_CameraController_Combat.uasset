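; Combat camera controller that pans the view and handles operator deployment and click interaction.
; After a start delay, Tick converts left-mouse drag into swept world offsets on the Sphere component.
; Left clicks trace from the cursor, switching I_Interactable focus between hit actors.
; SpawnOperatorFromClass spawns one selected operator from passed data, which input actions then place, rotate in four directions, confirm or cancel.
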(event Custom|Start%20Level
  (bind _returnvalue (Game|GetPlayerController 0))
  ;[0.04062 0.04062 0.04062] Start Level After Delay
  (Utilities|FlowControl|Delay 4.0)
  (bind _output_get (Variables|/Script/Engine.PlayerController|SetbShowMouseCursor _returnvalue true))
  (Variables|/Script/Engine.PlayerController|SetbEnableTouchEvents _returnvalue _output_get)
  (Variables|Default|Setlevel%20started%20? true))

(event EventBeginPlay
  (CallFunction|StartLevel))

(event EventTick
  (params (DeltaSeconds :type Float%20%28single-precision%29))
  (CallFunction|DragMovement))

(event Input|ActionEvents|InputActionLeftClick
  (params (Key :type Key%20Structure :default "None"))
  (:Pressed
    (bind _returnvalue (Class|WidgetLayoutLibrary|GetMousePositiononViewport))
    (Variables|Default|SetprevieousTouchLocation _returnvalue)
    (CallFunction|InteractwithObjectonClick)))

(event Input|ActionEvents|InputActionRightClick
  (params (Key :type Key%20Structure :default "None"))
  (bind _selected_operator (Variables|Default|Getselected%20operator))
  (:Pressed
    (Utilities|IsValid _selected_operator
      (:Is%20Valid
        (if (not (Variables|/Game/Operators/Blueprints/BP_Operator_2D.BP_Operator_2D_C|Gethas%20been%20placed? _selected_operator))
          (Default|PlaceOperator _selected_operator))))))

(event Input|ActionEvents|InputActionConfirmPlacement
  (params (Key :type Key%20Structure :default "None"))
  (bind _selected_operator (Variables|Default|Getselected%20operator))
  (:Pressed
    (Utilities|IsValid _selected_operator
      (:Is%20Valid
        (if (Variables|/Game/Operators/Blueprints/BP_Operator_2D.BP_Operator_2D_C|Gethas%20been%20placed? _selected_operator)
          (Default|FinishDeployment _selected_operator))))))

(event Input|ActionEvents|InputActionCancelPlacement
  (params (Key :type Key%20Structure :default "None"))
  (:Pressed
    (Utilities|IsValid (Variables|Default|Getselected%20operator)
      (:Is%20Valid
        (Default|CancelDeployment (Variables|Default|Getselected%20operator))
        (Variables|Default|Setselected%20operator 0)))))

(event Custom|Drag%20Movement
  ;[0.04062 0.04062 0.04062] Mvement Handler
  (if (Variables|Default|Getlevel%20started%20?)
    (if (Game|Player|IsInputKeyDown (Game|GetPlayerController 0) "LeftMouseButton")
      (bind _returnvalue (Class|WidgetLayoutLibrary|GetMousePositiononViewport))
      (Variables|Default|SetnewTouchLocation _returnvalue)
      (Transformation|AddWorldOffset (Variables|Default|GetSphere) (Math|Vector|MakeVector (.y (- (Variables|Default|GetnewTouchLocation) (Variables|Default|GetprevieousTouchLocation))) (* (.x (- (Variables|Default|GetnewTouchLocation) (Variables|Default|GetprevieousTouchLocation))) -1.0) 0.0) true false)
      (Variables|Default|SetprevieousTouchLocation (Variables|Default|GetnewTouchLocation)))))

(event Custom|Rotate%20Operator
  (params (New%20Rotation :type Float%20%28single-precision%29))
  (bind _selected_operator (Variables|Default|Getselected%20operator))
  (Utilities|IsValid _selected_operator
    (:Is%20Valid
      (Default|RotateOperator _selected_operator New%20Rotation))))

(event Input|ActionEvents|InputActionUp
  (params (Key :type Key%20Structure))
  (:Pressed
    (CallFunction|RotateOperator 0.0)))

(event Input|ActionEvents|InputActionDown
  (params (Key :type Key%20Structure))
  (:Pressed
    (CallFunction|RotateOperator 1.8e+02)))

(event Input|ActionEvents|InputActionLeft
  (params (Key :type Key%20Structure))
  (:Pressed
    (CallFunction|RotateOperator -9e+01)))

(event Input|ActionEvents|InputActionRight
  (params (Key :type Key%20Structure))
  (:Pressed
    (CallFunction|RotateOperator 9e+01)))

(event Custom|Spawn%20Operator%20From%20Class
  (params (data :type Struct%20Runtime%20Operator%20Structure))
  (bind (_operatorclass _redeploycount _level _selectedskill) (Utilities|Struct|BreakStruct_RuntimeOperator data))
  ;[0.04062 0.04062 0.04062] Spawn Operator
  (Utilities|IsValid (Variables|Default|Getselected%20operator)
    (:Is%20Not%20Valid
      (Actor|GetAllActorsOfClass _operatorclass)
      (bind _returnvalue (Game|SpawnActorfromClass _operatorclass (Math|Transform|MakeTransform "0.000000,0.000000,20000.000000" "0, 0, 0" "1.000000,1.000000,1.000000") "Undefined" "MultiplyWithRoot" 0 _redeploycount _level _selectedskill 0))
      (Variables|Default|Setselected%20operator _returnvalue))))

(event Custom|Interact%20With%20Object%20On%20Click
  ;[0.04062 0.04062 0.04062] Interact
  (bind (_hit_location _hit _hit_actor) (CallFunction|LineTracefromCursor 0 "TraceTypeQuery1" "None"))
  (if _hit
    (if (not (== _hit_actor (Variables|Default|Getinteracted%20actor)))
      (Utilities|IsValid (Variables|Default|Getinteracted%20actor)
        (:Is%20Valid
          (bind _asi_interactable (Utilities|Casting|CastToI_Interactable (Variables|Default|Getinteracted%20actor)))
          (Default|EndInteraction _asi_interactable _hit_actor))
        (:Is%20Not%20Valid
          _))
      (bind _asi_interactable_2 (Utilities|Casting|CastToI_Interactable _hit_actor)
        (:then
          (Default|Interact _asi_interactable_2 _hit_actor)
          (Variables|Default|Setinteracted%20actor _hit_actor))
        (:CastFailed
          (Variables|Default|Setinteracted%20actor 0))))))

(fn ConstructionScript)

(fn LineTracefromCursor
  (params (actors%20to%20ignore :type Array%20of%20Actor%20Object%20References) (Trace%20channel :type ETraceTypeQuery%20Enum :default "TraceTypeQuery1") (DrawDebugType :type EDrawDebugTrace%20Enum :default "None"))
  (bind _returnvalue (Game|GetPlayerController 0))
  (bind (_worldlocation _worlddirection) (Game|Player|ConvertMouseLocationToWorldSpace _returnvalue))
  (bind (_outhit _returnvalue_2) (Collision|LineTraceByChannel _worldlocation (+ _worldlocation (* _worlddirection 1e+04)) Trace%20channel false actors%20to%20ignore DrawDebugType))
  (return (.Location (Collision|BreakHitResult _outhit)) _returnvalue_2 (.HitActor (Collision|BreakHitResult _outhit)) (.HitComponent (Collision|BreakHitResult _outhit)) (.HitItem (Collision|BreakHitResult _outhit))))