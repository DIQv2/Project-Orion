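; Cancel button actor for the travel objective point menu, used as a child actor of BP_ObjectivePoint.
; Its Interact function casts the parent actor to BP_ObjectivePoint, calls CloseMenu on it, plays a 2D notification sound and returns false.
; The event graph holds only disabled default events, so all behaviour lives in Interact.
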(event EventBeginPlay
  (|CallParentFunction) ; This node is disabled and will not be called.\nDrag off pins to build functionality.
)

(event Collision|EventActorBeginOverlap
  (params (OtherActor :type Actor%20Object%20Reference))
  (|CallParentFunction OtherActor) ; This node is disabled and will not be called.\nDrag off pins to build functionality.
)

(event EventTick
  (params (DeltaSeconds :type Float%20%28single-precision%29))
  (|CallParentFunction DeltaSeconds) ; This node is disabled and will not be called.\nDrag off pins to build functionality.
)

(fn ConstructionScript
  (|CallParentFunction))

(fn Interact
  (params (instigator :type Actor%20Object%20Reference))
  (bind _asbp_objective_point (Utilities|Casting|CastToBP_ObjectivePoint (Actor|GetParentActor)))
  (Default|CloseMenu _asbp_objective_point)
  (Audio|PlaySound2D "/Game/Gameplay/Travel/ObjectivePoint/SFX/mixkit-retro-arcade-casino-notification-211.mixkit-retro-arcade-casino-notification-211" 0.8 0.7 0.3 0 0)
  (return false))